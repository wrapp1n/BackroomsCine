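; BP_Whisper is an AI-controlled enemy character that kills a Backroomer player on contact.
; A Sphere overlap casts the other actor to BP_Backroomer and calls its OnPlayerDeath.
; UpdateState stores the new state, sets a slower walk speed for Normal and a shared faster one for Chase, Battle and Searching, then writes the state to the controller's Blackboard.
; The CurrentState OnRep handler is empty.
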(event `self.Sphere.OnComponentBeginOverlap`
  (params (OverlappedComponent :type "PrimitiveComponent Object Reference") (OtherActor :type "Actor Object Reference") (OtherComp :type "PrimitiveComponent Object Reference") (OtherBodyIndex :type Integer) (bFromSweep :type Boolean) (SweepResult :type "HitResult Structure (by ref)"))
  (bind _asbp_backroomer (cast `/Game/TheBackrooms/Blueprints/Characters/BP_Backroomer` OtherActor))
  (`/Game/TheBackrooms/Blueprints/Characters/BP_Backroomer.OnPlayerDeath` _asbp_backroomer))

(fn `OnRep_CurrentState`)

(fn `UpdateState`
  (params (NewState :type "/Game/TheBackrooms/Characters/Whisper/E_WhisperState Enum" :default "NewEnumerator0"))
  (bind _charactermovement (`self.CharacterMovement`))
  (bind _output_get (set `self.CurrentState` NewState))
  (switch `/Game/TheBackrooms/Characters/Whisper/E_WhisperState` _output_get
    (:`NewEnumerator0`
      (set `CharacterMovementComponent.MaxWalkSpeed` 350.0 _charactermovement))
    (:`NewEnumerator1`
      (set `CharacterMovementComponent.MaxWalkSpeed` 405.0 _charactermovement :!label _label))
    (:`NewEnumerator2`
      (goto _label))
    (:`NewEnumerator3`
      (goto _label)))
  (`BlackboardComponent.SetValueAsEnum` (`AIBlueprintHelperLibrary.GetBlackboard` (`self.GetController`)) "CurrentState" _output_get))

(fn `UserConstructionScript`)